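; Player blueprint that moves by input-driven local offsets without sweep and can pick up and drop physics objects.
; GrabBox input toggles between grabbing whatever a forward Visibility trace from the Cylinder hits and releasing it.
; A PhysicsHandle pulls the held object to the Mano component each Tick, while the trace also redraws for debugging.
; Grabbing raises angular damping; dropping zeroes velocity and clears damping after a short delay.
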(event Custom|Grab
  ;[1 1 1] GrabBox
  (CallFunction|DrawLine)
  (if (stale Custom|DrawLine _returnvalue_2)
    (Variables|Default|SetPhysicsObject (.HitComponent (Collision|BreakHitResult (stale Custom|DrawLine _outhit))))
    (Class|PhysicsHandleComponent|GrabComponentatLocation (Variables|Default|GetPhysicsHandle) (.HitComponent (Collision|BreakHitResult (stale Custom|DrawLine _outhit))) "None" (.Location (Collision|BreakHitResult (stale Custom|DrawLine _outhit))))
    (Variables|Default|SetHolingBox true)
    (Collision|SetCollisionResponsetoChannel (Variables|Default|GetPhysicsObject) "ECC_Pawn" "ECR_Block")
    (Class|PrimitiveComponent|SetAngularDamping (Variables|Default|GetPhysicsObject) 1e+01)))

(event Custom|Drop
  (bind _physicsobject (Variables|Default|GetPhysicsObject))
  ;[1 1 1] Drop Box
  (Physics|Components|PhysicsHandle|ReleaseComponent (Variables|Default|GetPhysicsHandle))
  (Variables|Default|SetHolingBox false)
  (Collision|SetCollisionResponsetoChannel _physicsobject "ECC_Pawn" "ECR_Block")
  (Class|PrimitiveComponent|SetAllPhysicsLinearVelocity _physicsobject "0, 0, 0" false)
  (Utilities|FlowControl|Delay 0.2)
  (Class|PrimitiveComponent|SetAngularDamping _physicsobject 0.0))

(event Custom|DrawLine
  (bind _cylinder (Variables|Default|GetCylinder))
  (bind _returnvalue (Transformation|GetWorldLocation _cylinder))
  ;[1 1 1] Line Trace
  (bind (_outhit _returnvalue_2) (Collision|LineTraceByChannel _returnvalue (+ _returnvalue (* (Math|Vector|GetForwardVector (Transformation|GetWorldRotation _cylinder)) 1e+03)) "TraceTypeQuery1" false 0 "ForOneFrame")))

(event EventTick
  (params (DeltaSeconds :type Float%20%28single-precision%29))
  ;[1 1 1] Event Tick
  (CallFunction|DrawLine)
  (Physics|Components|PhysicsHandle|SetTargetLocation (Variables|Default|GetPhysicsHandle) (Transformation|GetWorldLocation (Variables|Default|GetMano))))

(event Input|ActionEvents|InputActionGrabBox
  (params (Key :type Key%20Structure))
  ;[1 1 1] Grab And Drop Box
  (:Pressed
    (if (Variables|Default|GetHolingBox)
      (CallFunction|Drop)
      (else
        (CallFunction|Grab)))))

(event Input|AxisEvents|InputAxisMoveForward
  (params (AxisValue :type Float%20%28single-precision%29))
  ;[1 1 1] Movement
  (Transformation|AddActorLocalOffset (Math|Vector|MakeVector (* AxisValue (Variables|Default|GetForwardSpeed)) 0.0 0.0) false false))

(event Input|AxisEvents|InputAxisMoveRight
  (params (AxisValue :type Float%20%28single-precision%29))
  ;[1 1 1] Movement
  (Transformation|AddActorLocalOffset (Math|Vector|MakeVector 0.0 (* AxisValue (Variables|Default|GetRightSpeed)) 0.0) false false))

(fn ConstructionScript)