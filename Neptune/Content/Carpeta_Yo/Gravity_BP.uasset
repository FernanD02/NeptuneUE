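; Gravity source Blueprint that pulls every actor implementing Gravity_Interface_BP toward its own location.
; Each Tick moves those actors with a swept offset scaled by Intensity, without delta time, so pull speed depends on frame rate.
; A debug-drawn Visibility trace runs from the source to each actor, and on a hit aligns the actor's up axis to the impact normal while using its forward vector as heading.
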(event EventTick
  (params (DeltaSeconds :type Float%20%28single-precision%29))
  (bind _returnvalue (Transformation|GetWorldLocation))
  ;[1 1 1] Gravity
  (bind _outactors (Actor|GetAllActorswithInterface "/Game/Carpeta_Yo/Gravity_Interface_BP.Gravity_Interface_BP_C"))
  (for _array_element _outactors
    (Transformation|AddActorWorldOffset _array_element (* (Math|Vector|Normalize (- _returnvalue (Transformation|GetActorLocation _array_element))) (* (Variables|Default|GetIntensity) 0.01)) true)
    (bind (_outhit _returnvalue_2) (Collision|LineTraceByChannel _returnvalue (Transformation|GetActorLocation _array_element) "TraceTypeQuery1" false 0 "ForOneFrame" false "(R=1.000000,G=0.000000,B=0.000000,A=1.000000)" "(R=0.099045,G=0.000000,B=1.000000,A=1.000000)"))
    (if _returnvalue_2
      (Transformation|SetActorRotation _array_element (Math|Rotator|MakeRotfromZX (.ImpactNormal (Collision|BreakHitResult _outhit)) (Transformation|GetActorForwardVector _array_element))))))